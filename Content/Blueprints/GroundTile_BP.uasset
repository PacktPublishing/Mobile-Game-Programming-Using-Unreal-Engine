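; Endless-runner ground tile that fills its three lanes with random obstacles, coins and powerups on BeginPlay.
; Each lane runs chained range checks that re-roll each time, so spawn odds differ from the range widths; walls appear only in outer lanes.
; When the character hits its Box, it has the game mode spawn tiles, adds points, multiplies walk speed within a clamp, then destroys itself after a delay.
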(event `self.ReceiveBeginPlay`
  (`self.SpawnObstacles`))

(event `self.Box.OnComponentBeginOverlap`
  (params (OverlappedComponent :type "PrimitiveComponent Object Reference") (OtherActor :type "Actor Object Reference") (OtherComp :type "PrimitiveComponent Object Reference") (OtherBodyIndex :type Integer) (bFromSweep :type Boolean) (SweepResult :type "HitResult Structure (by ref)"))
  (cast `/Game/ThirdPersonBP/Blueprints/ThirdPersonCharacter` OtherActor)
  (bind _asthird_person_game_mode (cast `/Game/ThirdPersonBP/Blueprints/ThirdPersonGameMode` (`GameplayStatics.GetGameMode`)))
  (`/Game/ThirdPersonBP/Blueprints/ThirdPersonGameMode.SpawnGroundTiles` _asthird_person_game_mode)
  (bind _asthird_person_game_mode_2 (cast `/Game/ThirdPersonBP/Blueprints/ThirdPersonGameMode` (`GameplayStatics.GetGameMode`)))
  (set `/Game/ThirdPersonBP/Blueprints/ThirdPersonGameMode.CurrentPoints` (+ (`/Game/ThirdPersonBP/Blueprints/ThirdPersonGameMode.CurrentPoints` _asthird_person_game_mode_2) 10) _asthird_person_game_mode_2)
  (bind _asthird_person_character (cast `/Game/ThirdPersonBP/Blueprints/ThirdPersonCharacter` (`GameplayStatics.GetPlayerCharacter` 0)))
  (bind _charactermovement (`Character.CharacterMovement` _asthird_person_character))
  (set `CharacterMovementComponent.MaxWalkSpeed` (`KismetMathLibrary.FClamp` (* (`CharacterMovementComponent.MaxWalkSpeed` _charactermovement) (`self.SpeedMultiplicationFactor`)) 600.0 (`self.MaxSpeed`)) _charactermovement)
  (`KismetSystemLibrary.Delay` 2.0)
  (`self.K2_DestroyActor`))

(fn `SpawnObstacles`
  (bind _returnvalue (`KismetMathLibrary.RandomFloatInRange` 0.0 1.0))
  (bind _returnvalue_2 (`KismetMathLibrary.RandomFloatInRange` 0.0 1.0))
  (bind _returnvalue_3 (`KismetMathLibrary.RandomFloatInRange` 0.0 1.0))
  (bind _returnvalue_4 (`SceneComponent.K2_GetComponentToWorld` (`self.Lane0`)))
  (bind _returnvalue_5 (`SceneComponent.K2_GetComponentToWorld` (`self.Lane2`)))
  (bind _returnvalue_6 (`SceneComponent.K2_GetComponentToWorld` (`self.Lane1`)))
  ;[1 1 1] Lane 0
  (if (`KismetMathLibrary.InRange_FloatFloat` _returnvalue_3 0.0 0.05)
    _
    (elif (`KismetMathLibrary.InRange_FloatFloat` _returnvalue_3 0.05 0.3)
      (`|SpawnActorFromClass` "/Game/Blueprints/Obstacles/BP_PicketFence.BP_PicketFence_C" _returnvalue_4 "Undefined" "OverrideRootScale" null null)
      (elif (`KismetMathLibrary.InRange_FloatFloat` _returnvalue_3 0.3 0.45)
        (`|SpawnActorFromClass` "/Game/Blueprints/Obstacles/BP_PizzaSign.BP_PizzaSign_C" _returnvalue_4 "Undefined" "OverrideRootScale" null null)
        (elif (`KismetMathLibrary.InRange_FloatFloat` _returnvalue_3 0.45 0.55)
          (`|SpawnActorFromClass` "/Game/Blueprints/Obstacles/BP_WallLeft.BP_WallLeft_C" _returnvalue_4 "Undefined" "OverrideRootScale" null null)
          (elif (`KismetMathLibrary.InRange_FloatFloat` _returnvalue_3 0.55 0.9)
            (`|SpawnActorFromClass` "/Game/Blueprints/Pickups/BP_Coin.BP_Coin_C" _returnvalue_4 "Undefined" "OverrideRootScale" null null)
            (elif (`KismetMathLibrary.InRange_FloatFloat` _returnvalue_3 0.9 0.95)
              (`|SpawnActorFromClass` "/Game/Blueprints/Pickups/BP_CoinMagnet.BP_CoinMagnet_C" _returnvalue_4 "Undefined" "OverrideRootScale" null null)
              (elif (`KismetMathLibrary.InRange_FloatFloat` _returnvalue_3 0.95)
                (`|SpawnActorFromClass` "/Game/Blueprints/Pickups/BP_JumpPowerup.BP_JumpPowerup_C" _returnvalue_4 "Undefined" "OverrideRootScale" null null))))))))
  ;[1 1 1] Lane 1
  (if (`KismetMathLibrary.InRange_FloatFloat` _returnvalue_2 0.0 0.05)
    _
    (elif (`KismetMathLibrary.InRange_FloatFloat` _returnvalue_2 0.05 0.25)
      (`|SpawnActorFromClass` "/Game/Blueprints/Obstacles/BP_PicketFence.BP_PicketFence_C" _returnvalue_6 "Undefined" "OverrideRootScale" null null)
      (elif (`KismetMathLibrary.InRange_FloatFloat` _returnvalue_2 0.25 0.35)
        (`|SpawnActorFromClass` "/Game/Blueprints/Obstacles/BP_PizzaSign.BP_PizzaSign_C" _returnvalue_6 "Undefined" "OverrideRootScale" null null)
        (elif (`KismetMathLibrary.InRange_FloatFloat` _returnvalue_2 0.35 0.55)
          (`|SpawnActorFromClass` "/Game/Blueprints/Pickups/BP_Coin.BP_Coin_C" _returnvalue_6 "Undefined" "OverrideRootScale" null null)
          (elif (`KismetMathLibrary.InRange_FloatFloat` _returnvalue_2 0.55 0.9)
            (`|SpawnActorFromClass` "/Game/Blueprints/Pickups/BP_Coin.BP_Coin_C" _returnvalue_6 "Undefined" "OverrideRootScale" null null)
            (elif (`KismetMathLibrary.InRange_FloatFloat` _returnvalue_2 0.9 0.95)
              (`|SpawnActorFromClass` "/Game/Blueprints/Pickups/BP_CoinMagnet.BP_CoinMagnet_C" _returnvalue_6 "Undefined" "OverrideRootScale" null null)
              (elif (`KismetMathLibrary.InRange_FloatFloat` _returnvalue_2 0.95)
                (`|SpawnActorFromClass` "/Game/Blueprints/Pickups/BP_JumpPowerup.BP_JumpPowerup_C" _returnvalue_6 "Undefined" "OverrideRootScale" null null))))))))
  ;[1 1 1] Lane2
  (if (`KismetMathLibrary.InRange_FloatFloat` _returnvalue 0.0 0.05)
    _
    (elif (`KismetMathLibrary.InRange_FloatFloat` _returnvalue 0.05 0.35)
      (`|SpawnActorFromClass` "/Game/Blueprints/Obstacles/BP_PicketFence.BP_PicketFence_C" _returnvalue_5 "Undefined" "OverrideRootScale" null null)
      (elif (`KismetMathLibrary.InRange_FloatFloat` _returnvalue 0.35 0.5)
        (`|SpawnActorFromClass` "/Game/Blueprints/Obstacles/BP_PizzaSign.BP_PizzaSign_C" _returnvalue_5 "Undefined" "OverrideRootScale" null null)
        (elif (`KismetMathLibrary.InRange_FloatFloat` _returnvalue 0.5 0.6)
          (`|SpawnActorFromClass` "/Game/Blueprints/Obstacles/BP_WallRight.BP_WallRight_C" _returnvalue_5 "Undefined" "OverrideRootScale" null null)
          (elif (`KismetMathLibrary.InRange_FloatFloat` _returnvalue 0.6 0.9)
            (`|SpawnActorFromClass` "/Game/Blueprints/Pickups/BP_Coin.BP_Coin_C" _returnvalue_5 "Undefined" "OverrideRootScale" null null)
            (elif (`KismetMathLibrary.InRange_FloatFloat` _returnvalue 0.9 0.95)
              (`|SpawnActorFromClass` "/Game/Blueprints/Pickups/BP_CoinMagnet.BP_CoinMagnet_C" _returnvalue_5 "Undefined" "OverrideRootScale" null null)
              (elif (`KismetMathLibrary.InRange_FloatFloat` _returnvalue 0.95)
                (`|SpawnActorFromClass` "/Game/Blueprints/Pickups/BP_JumpPowerup.BP_JumpPowerup_C" _returnvalue_5 "Undefined" "OverrideRootScale" null null)))))))))

(fn `UserConstructionScript`)